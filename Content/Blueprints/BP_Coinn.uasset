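; BP_Coinn is a coin pickup actor that calls CoinGet on BP_ThirdPersonCharacter when that character overlaps its Coin component.
; The overlap then casts the game mode to GM_SavLoad, printing an error on failure and doing nothing further on success.
; LoadState calls CollectThyself, which marks the coin by switching its material to Glass.
; The logic that records the coin in the save state's AlteredActors and destroys it is disconnected.
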(event `/Game/Blueprints/BPI_LevelActorSaveable.LoadState`
  (`self.CollectThyself`))

(event `CollectThyself`
  (`PrimitiveComponent.SetMaterial` (`self.Coin`) 0 "/DatasmithContent/Materials/FBXImporter/VRED/Glass.Glass"))

(event `self.Coin.OnComponentBeginOverlap`
  (params (OverlappedComponent :type "PrimitiveComponent Object Reference") (OtherActor :type "Actor Object Reference") (OtherComp :type "PrimitiveComponent Object Reference") (OtherBodyIndex :type Integer) (bFromSweep :type Boolean) (SweepResult :type "HitResult Structure (by ref)"))
  ; When run into,
  ; was it the player?
  ; if so, find the game mode
  ; add myself to the SG_LevelState savegame array for collected coins
  ; and delete myself.
  (bind _asbp_third_person_character (cast `/Game/ThirdPerson/Blueprints/BP_ThirdPersonCharacter` OtherActor))
  (`/Game/ThirdPerson/Blueprints/BP_ThirdPersonCharacter.CoinGet` _asbp_third_person_character)
  (cast `/Game/Blueprints/SavingLoading/GM_SavLoad` (`GameplayStatics.GetGameMode`)
    (:`CastFailed`
      (`KismetSystemLibrary.PrintString` "WRONG GAME MODE"))))

(fn `UserConstructionScript`)