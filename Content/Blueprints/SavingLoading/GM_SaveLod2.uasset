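; Game mode, judging by its GM prefix, that loads and saves per-level state, including which coins are collected.
; On BeginPlay it loads the SG_LevelStatee save from a slot named after the current level, or creates a new save object if none exists.
; Loaded coin references that are valid get CollectThyself called to restore their collected state.
; SaveLevelStateToFile writes the object back to the same slot and prints the result.
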(event `self.ReceiveBeginPlay`
  (`self.Load Level State From File`))

(event `Load Level State From File`
  (bind _returnvalue (`GameplayStatics.GetCurrentLevelName` true))
  (bind _returnvalue_2 (`GameplayStatics.DoesSaveGameExist` _returnvalue))
  (if _returnvalue_2
    (bind _returnvalue_3 (`GameplayStatics.LoadGameFromSlot` _returnvalue))
    (bind _assg_level_statee (cast `/Game/Blueprints/SavingLoading/SG_LevelStatee` _returnvalue_3)
      (:`then`
        (set `self.SG_LevelStatee` _assg_level_statee)
        (`KismetSystemLibrary.PrintString` "Loaded existing level state")
        ; load collected coins
        (for _array_element (`/Game/Blueprints/SavingLoading/SG_LevelStatee.CollectedCoins` (`self.SG_LevelStatee`))
          (`/Engine/EditorBlueprintResources/StandardMacros.IsValid` _array_element ; maybe teh coin is in a different level?\nif so, ignore it
            (:`Is Valid`
              (`/Game/Blueprints/BP_Coinn.CollectThyself` _array_element)))))
      (:`CastFailed`
        (`KismetSystemLibrary.PrintString` "cast failed")))
    (else
      (bind _returnvalue_4 (`GameplayStatics.CreateSaveGameObject` "/Game/Blueprints/SavingLoading/SG_LevelStatee.SG_LevelStatee_C"))
      (set `self.SG_LevelStatee` _returnvalue_4)
      (`KismetSystemLibrary.PrintString` "new save game for level state has been created"))))

(event `SaveLevelStateToFile`
  (bind _returnvalue (`GameplayStatics.GetCurrentLevelName` true))
  (bind _returnvalue_2 (`GameplayStatics.SaveGameToSlot` (`self.SG_LevelStatee`) _returnvalue))
  (if _returnvalue_2
    (`KismetSystemLibrary.PrintText` "Level State Saved" true true (struct :`R` 0.321655 :`G` 1.0 :`B` 0.013734 :`A` 1.0) 5.0)
    (else
      (`KismetSystemLibrary.PrintText` "Level State Failed To Save" true true (struct :`R` 1.0 :`B` 0.03001 :`A` 1.0) 5.0))))

(fn `UserConstructionScript`)